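; BP_HealthPowerup is a space shooter pickup that grants extra lives to the player character.
; On actor overlap it calls the parent handler, then casts the other actor to BP_SpaceSCharacter.
; A successful cast calls IncreaseLifes with a small random amount, and the powerup destroys itself after a brief delay.
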(event EventBeginPlay
  (|CallParentFunction) ; This node is disabled and will not be called.\nDrag off pins to build functionality.
)

(event Collision|EventActorBeginOverlap
  (params (OtherActor :type Actor%20Object%20Reference))
  (|CallParentFunction OtherActor)
  (bind _asbp_space_scharacter (Utilities|Casting|CastToBP_SpaceSCharacter OtherActor))
  (Default|IncreaseLifes _asbp_space_scharacter (Math|Random|RandomIntegerinRange 2 5))
  (Utilities|FlowControl|Delay 0.1)
  (Actor|DestroyActor))

(event EventTick
  (params (DeltaSeconds :type Float%20%28single-precision%29))
  (|CallParentFunction DeltaSeconds) ; This node is disabled and will not be called.\nDrag off pins to build functionality.
)

(fn ConstructionScript
  (|CallParentFunction))