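; BP_Powerup is a powerup actor for the space shooter that drifts across the XY plane and destroys itself after a set lifetime.
; BeginPlay picks a random positive X/Y direction, and Tick moves the actor along it without sweep until the timer reaches SpamLife.
; Overlapping an actor tagged "Lateral" bounces it by randomly jittering, normalizing and reversing the direction.
; No pickup effect is implemented here.
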(event EventBeginPlay
  (Variables|Default|SetDirection (Math|Vector|MakeVector (Math|Random|RandomFloat) (Math|Random|RandomFloat) 0.0)))

(event Collision|EventActorBeginOverlap
  (params (OtherActor :type Actor%20Object%20Reference))
  (CallFunction|Bounce OtherActor))

(event EventTick
  (params (DeltaSeconds :type Float%20%28single-precision%29))
  (bind _output_get (Variables|Default|SetTimer (+ DeltaSeconds (Variables|Default|GetTimer))))
  (if (>= _output_get (Variables|Default|GetSpamLife))
    (Actor|DestroyActor)
    (else
      (Transformation|SetActorLocation (+ (Transformation|GetActorLocation) (* (Variables|Default|GetDirection) (* DeltaSeconds (Variables|Default|GetSpeed)))) false false))))

(fn ConstructionScript)

(fn Bounce
  (params (Actor :type Actor%20Object%20Reference))
  (if (Utilities|Array|ContainsItem (Variables|/Script/Engine.Actor|GetTags Actor) "Lateral")
    (bind _value (CallFunction|GetRandomAxisValue (.x (Variables|Default|GetDirection))))
    (bind _value_2 (CallFunction|GetRandomAxisValue (.y (Variables|Default|GetDirection))))
    (Variables|Default|SetDirection (* (Math|Vector|Normalize (Math|Vector|MakeVector _value _value_2 0.0)) -1))))

(fn GetRandomAxisValue
  (params (AxisValue :type Float%20%28double-precision%29))
  (return (Math|Random|RandomFloatinRange (- AxisValue 0.5) (+ AxisValue 0.5))))