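; BP_RandomGenerator is the space shooter's enemy spawner, running on a looping timer set at BeginPlay.
; Each tick of that timer spawns a random one of three enemy classes at a random SpawnPoint-tagged component.
; The level-based type passed to GetClassToSpawn is ignored.
; Destroyed enemies that cast to BP_Enemy1 reduce SpawnTime, but the running timer is never reset to use it.
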(event Custom|Spawn
  (bind _enemyspawned (CallFunction|SpawnEnemy))
  (bind _asbp_enemy_1 (Utilities|Casting|CastToBP_Enemy1 _enemyspawned))
  (EventDispatchers|BindEventtoOnEnemyDestroy _asbp_enemy_1 (delegate Custom|EnemyDestroyed)))

(event Custom|EnemyDestroyed
  (Variables|Default|SetSpawnTime (- (Variables|Default|GetSpawnTime) 0.1)))

(event EventBeginPlay
  (Utilities|Time|SetTimerbyEvent (delegate Custom|Spawn) (Variables|Default|GetSpawnTime) true)
  (bind _asss_game_mode (Utilities|Casting|CastToSS_GameMode (Game|GetGameMode)))
  (Variables|Default|Setm_GameMode _asss_game_mode))

(event Collision|EventActorBeginOverlap
  (params (OtherActor :type Actor%20Object%20Reference)))

(event EventTick
  (params (DeltaSeconds :type Float%20%28single-precision%29)))

(fn ConstructionScript)

(fn SpawnEnemy
  (bind _returnvalue (Actor|GetComponentsbyTag "/Script/Engine.SceneComponent" "SpawnPoint"))
  (bind _class (CallFunction|GetClasstoSpawn (Math|Random|RandomInteger (Variables|/Game/00_SpaceShooter/SS_GameMode.SS_GameMode_C|GetLevel (Variables|Default|Getm_GameMode)))))
  (bind _returnvalue_2 (Game|SpawnActorfromClass _class (Transformation|GetWorldTransform (Utilities|Array|Get(acopy) _returnvalue (Math|Random|RandomInteger (Utilities|Array|Length _returnvalue)))) "Undefined" "MultiplyWithRoot" 0 0))
  (return _returnvalue_2))

(fn GetClasstoSpawn
  (params (Type :type Integer))
  (return (Utilities|Select :Index (Math|Integer|Clamp(Integer) (Math|Random|RandomIntegerinRange 0 2) 0 2) :Option%200 "/Game/00_SpaceShooter/Enemies/BP_Enemy1.BP_Enemy1_C" :Option%201 "/Game/00_SpaceShooter/Enemies/BP_Enemy2.BP_Enemy2_C" :Option%202 "/Game/00_SpaceShooter/Enemies/BP_Enemy3.BP_Enemy3_C")))