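; Player character for the space shooter, handling Enhanced Input movement, timer-gated firing, lives and a temporary shield.
; Shoot level sets how many fire points spawn ammo, and higher levels also shorten the fire delay.
; Overlapping an Enemy-tagged actor while unshielded costs lives and a shoot level, and running out notifies SS_GameMode of player death.
; The timed shield blocks that damage and blinks through a looping timer before it expires.
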(event Custom|UpdateFire
  (Variables|Default|SetCanFire true))

(event Custom|DamageActor
  (bind _output_get (Variables|Default|SetLifes (- (Variables|Default|GetLifes) 5)))
  (if (<= _output_get 0)
    (bind _asss_game_mode (Utilities|Casting|CastToSS_GameMode (Game|GetGameMode)))
    (Default|PlayerDead _asss_game_mode)))

(event Custom|IncreaseLifes
  (params (Life :type Integer))
  (Variables|Default|SetLifes (+ Life (Variables|Default|GetLifes))))

(event Custom|TurnOnShield
  (bind _shield (Variables|Default|GetShield))
  (if (not (Variables|Default|GetHasShield))
    (Variables|Default|SetHasShield true)
    (Rendering|SetVisibility _shield true false)
    (Utilities|FlowControl|Delay 7.0)
    (Utilities|Time|SetTimerbyFunctionName 0 "ToggleShieldVisibility" 0.2 true)
    (Utilities|FlowControl|Delay 3.0)
    (Utilities|Time|ClearTimerbyFunctionName 0 "ToggleShieldVisibility")
    (Variables|Default|SetHasShield false)
    (Rendering|SetVisibility _shield false false)))

(event Custom|DecreaseShootLevel
  (if (> (Variables|Default|GetShootLevel) 0)
    (bind _output_get (Variables|Default|SetShootLevel (- (Variables|Default|GetShootLevel) 1)))
    (if (< _output_get 3)
      (Variables|Default|SetFireDelay 0.5))))

(event Custom|IncreaseShootLevel
  (if (<= (Variables|Default|GetShootLevel) 3)
    (bind _output_get (Variables|Default|SetShootLevel (+ (Variables|Default|GetShootLevel) 1)))
    (if (>= _output_get 3)
      (Variables|Default|SetFireDelay 0.25))))

(event Input|EnhancedActionEvents|EnhancedInputActionBP_InputMove
  (params (ActionValue :type Vector%202D%20Structure) (ElapsedSeconds :type Float%20%28double-precision%29) (TriggeredSeconds :type Float%20%28double-precision%29) (InputAction :type Input%20Action%20Object%20Reference :default "/Game/00_SpaceShooter/Input/BP_InputMove.BP_InputMove"))
  (Pawn|Input|AddMovementInput (Transformation|GetActorRightVector) (.x ActionValue) false)
  (Pawn|Input|AddMovementInput (Transformation|GetActorForwardVector) (.y ActionValue) false))

(event Input|EnhancedActionEvents|EnhancedInputActionBP_InputFire
  (params (ActionValue :type Boolean) (ElapsedSeconds :type Float%20%28double-precision%29) (TriggeredSeconds :type Float%20%28double-precision%29) (InputAction :type Input%20Action%20Object%20Reference :default "/Game/00_SpaceShooter/Input/BP_InputFire.BP_InputFire"))
  (if (Variables|Default|GetCanFire)
    (CallFunction|DoFire)
    (Variables|Default|SetCanFire false)
    (Utilities|Time|SetTimerbyEvent (delegate Custom|UpdateFire) (Variables|Default|GetFireDelay))))

(event EventBeginPlay
  (bind _asplayer_controller (Utilities|Casting|CastToPlayerController (Pawn|GetController)))
  (Utilities|IsValid (PlayerController|LocalPlayerSubsystems|GetEnhancedInputLocalPlayerSubsystem _asplayer_controller)
    (:Is%20Valid
      (Input|AddMappingContext (PlayerController|LocalPlayerSubsystems|GetEnhancedInputLocalPlayerSubsystem _asplayer_controller) "/Game/00_SpaceShooter/Input/BP_InputMapping.BP_InputMapping" 0 "(bIgnoreAllPressedKeysUntilRelease=True,bForceImmediately=False,bNotifyUserSettings=False)")
      (Rendering|SetVisibility (Variables|Default|GetShield) false false))))

(event Collision|EventActorBeginOverlap
  (params (OtherActor :type Actor%20Object%20Reference))
  (if (Utilities|IsValid OtherActor)
    (if (not (Variables|Default|GetHasShield))
      (if (Utilities|Array|ContainsItem (Variables|/Script/Engine.Actor|GetTags OtherActor) "Enemy")
        (CallFunction|DamageActor)
        (CallFunction|DecreaseShootLevel)))))

(event EventTick
  (params (DeltaSeconds :type Float%20%28single-precision%29)))

(fn ConstructionScript)

(fn DoFire
  (bind _ammo (Variables|Default|GetAmmo))
  (bind _firepoint0 (Variables|Default|GetFirePoint0))
  (bind _shootlevel (Variables|Default|GetShootLevel))
  (bind _firepoint1 (Variables|Default|GetFirePoint1))
  (bind _firepoint2 (Variables|Default|GetFirePoint2))
  (bind _returnvalue (Transformation|GetWorldTransform _firepoint0))
  (bind _returnvalue_2 (Transformation|GetWorldTransform _firepoint1))
  (bind _returnvalue_3 (Transformation|GetWorldTransform _firepoint2))
  (if (== _shootlevel 0)
    (Game|SpawnActorfromClass _ammo _returnvalue "Undefined" "MultiplyWithRoot" 0 0)
    (elif (== _shootlevel 1)
      (Game|SpawnActorfromClass _ammo _returnvalue_2 "Undefined" "MultiplyWithRoot" 0 0)
      (Game|SpawnActorfromClass _ammo _returnvalue_3 "Undefined" "MultiplyWithRoot" 0 0)
      (elif (>= _shootlevel 2)
        (Game|SpawnActorfromClass _ammo _returnvalue "Undefined" "MultiplyWithRoot" 0 0)
        (Game|SpawnActorfromClass _ammo _returnvalue_2 "Undefined" "MultiplyWithRoot" 0 0)
        (Game|SpawnActorfromClass _ammo _returnvalue_3 "Undefined" "MultiplyWithRoot" 0 0)))))

(fn ToggleShieldVisibility
  (bind _shield (Variables|Default|GetShield))
  (if (Variables|Default|GetHasShield)
    (Rendering|SetVisibility _shield (not (Rendering|IsVisible _shield)) false)))